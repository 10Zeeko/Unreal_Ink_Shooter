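; BP_InkMeter relays ink meter values for two teams to the player's HUD.
; On BeginPlay it binds to the ink meter update event and forwards each update through a multicast RPC.
; The multicast casts player controller 0's pawn to BP_InkPlayerCharacter and passes both team values to its HUD ink meter widget, doing nothing if the cast fails.
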(event Custom|RPC_Multicast_OnUpdate
  (params (A :type Integer) (B :type Integer))
  (bind _asbp_ink_player_character (Utilities|Casting|CastToBP_InkPlayerCharacter (Pawn|GetControlledPawn (Game|GetPlayerController 0))))
  (Default|UpdateInk (Variables|/Game/Blueprints/Player/BP_InkPlayerCharacter.BP_InkPlayerCharacter_C|GetmInkMeterWidgetHUD _asbp_ink_player_character) (Math|Conversions|ToFloat(Integer) A) (Math|Conversions|ToFloat(Integer) B)))

(event Custom|OnUpdate
  (params (Team1 :type Integer) (Team2 :type Integer))
  (CallFunction|RPCMulticastonUpdate Team1 Team2))

(event EventBeginPlay
  (EventDispatchers|BindEventtoEvonUpdateInkMeter (delegate Custom|OnUpdate)))

(fn ConstructionScript)